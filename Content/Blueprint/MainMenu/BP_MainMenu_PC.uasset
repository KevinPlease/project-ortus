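; BP_MainMenu_PC is the main menu player controller, handling the New Game and continent selection flow.
; It caches the game instance and starts in UI-only input.
; New Game plays a timeline that animates control rotation pitch, then switches to game-and-UI input.
; Selecting a continent restores UI-only input, prints the choice for debugging, and has the game instance open Level_Game with that continent.
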(event `self.ReceiveBeginPlay`
  ;[1 1 1] Begin Play for this actor Get references
  (bind _asbp_mgame_instance (cast `/Game/Blueprint/AllLevels/BP_MGameInstance` (`GameplayStatics.GetGameInstance`)))
  (set `self.GameInstanceRef` _asbp_mgame_instance)
  (`WidgetBlueprintLibrary.SetInputMode_UIOnlyEx` self null))

(event `On New Game Click`
  ;[1 1 1] On New Game selected
  (bind (_direction _newtrack_1) (`Timeline|Lerp Pawn Rotation` :!via `PlayFromStart`)
    (:`Update`
      (`self.SetControlRotation` (`KismetMathLibrary.MakeRotator` 0.0 (.y _newtrack_1))))
    (:`Finished`
      (`WidgetBlueprintLibrary.SetInputMode_GameAndUIEx` self null))))

(event `On Continent Selection`
  (params (Selection :type "/Game/Data/Enums/Enum_Continents Enum" :default "NewEnumerator0"))
  ;[1 1 1] Continent selected
  (`WidgetBlueprintLibrary.SetInputMode_UIOnlyEx` self null)
  (switch `/Game/Data/Enums/Enum_Continents` Selection
    (:`NewEnumerator0`
      (`KismetSystemLibrary.PrintString` "USA"))
    (:`NewEnumerator1`
      (`KismetSystemLibrary.PrintString` "Europe"))
    (:`NewEnumerator2`
      (`KismetSystemLibrary.PrintString` "Other")))
  (`/Game/Blueprint/AllLevels/BP_MGameInstance.Open Level With Continent` (`self.GameInstanceRef`) Selection "Level_Game"))

(fn `UserConstructionScript`)