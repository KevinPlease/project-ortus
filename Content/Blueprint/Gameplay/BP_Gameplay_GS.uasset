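; Game state Blueprint for a country-management game, holding the calendar, countries and sectors.
; BeginPlay builds countries and sectors from data tables (save loading is a stub returning false), then initializes the game mode.
; Once the calendar starts, Tick converts speed-scaled time into clock and date, passes the date to the game mode and triggers monthly country progression.
; Helpers look up countries and total sector maintenance costs; several setters are stubs.
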(event `self.ReceiveBeginPlay`
  ;[1 1 1] Game started - Load state here
  (bind _asbp_gameplay_gm (cast `/Game/Blueprint/Gameplay/BP_Gameplay_GM` (`GameplayStatics.GetGameMode`)))
  (set `self.GameModeRef` _asbp_gameplay_gm)
  (bind _isloaded (`self.LoadSavedGameState`))
  (if (not _isloaded)
    (`self.NewGameState`))
  (`/Game/Blueprint/Gameplay/BP_Gameplay_GM.Init Game Mode` (`self.GameModeRef`)))

(event `self.ReceiveTick`
  (params (DeltaSeconds :type "Float (single-precision)"))
  (bind (_clockwork _daytick) (`self.Get Clockwork` DeltaSeconds))
  ;[0.5972 0.2831 0.05286] TODO: Calendar System --- Should be converted to C++
  (set `self.Clockwork` _clockwork)
  (set `self.DayTick` _daytick)
  (`self.Update Clock`)
  (bind (_new_game_date _newmonth) (`self.Update Date`))
  (`/Game/Blueprint/Gameplay/BP_Gameplay_GM.Call Player Update DateTime` (`self.GameModeRef`) _new_game_date)
  (if _newmonth
    ;[1 1 1] Run monthly progression events
    (`/Game/Blueprint/Gameplay/BP_Gameplay_GM.Event Countries Progression - Monthly` (`self.GameModeRef`))))

(fn `Get Clockwork`
  (params (`Delta Seconds` :type "Float (double-precision)"))
  (returns (ClockWork :type "Float (double-precision)") (DayTick :type Integer))
  (bind (_remainder _returnvalue) (`KismetMathLibrary.FMod` (+ (/ `Delta Seconds` (`self.TimeUnit`)) (`self.Clockwork`)) (`self.HoursInDay`)))
  (return _remainder _returnvalue))

(fn `Get Info For Country`
  (params (Name :type String))
  (returns (CountrySelected :type "Country Object Reference"))
  (locals (SelectedCountry :type "Country Object Reference"))
  (for _array_element (`self.Countries`)
    (if (`KismetStringLibrary.EqualEqual_StrStr` (`Country.GetCountryName` _array_element) Name)
      (set `local.SelectedCountry` _array_element)
      (break)))
  (return (`local.SelectedCountry`)))

(fn `GetMaintenanceCosts`
  (returns (MaintenanceCosts :type "Float (double-precision)"))
  (locals (Costs :type "Float (double-precision)"))
  (for _array_element (`self.Sectors`)
    (set `local.Costs` (+ (`BasicSector.GetAllMaintenanceCosts` _array_element) (`local.Costs`))))
  (return (`local.Costs`)))

(fn `GetSelectedCountry`
  (returns (CountrySelected :type "Country Object Reference") (HasSelected :type Boolean))
  (bind _returnvalue (`KismetStringLibrary.NotEqual_StrStr` (`self.SelectedCountryName`)))
  (if _returnvalue
    _
    (else
      _))
  (return (`self.Get Info For Country` (`self.SelectedCountryName`)) _returnvalue))

(fn `Load Clock/Date`
  (params (Seconds :type Integer) (Minutes :type Integer) (Hours :type Integer))
  (set `self.Clockwork` (+ (`KismetMathLibrary.Conv_IntToDouble` Seconds) (`KismetMathLibrary.Conv_IntToDouble` Minutes) (`KismetMathLibrary.Conv_IntToDouble` Hours)))
  (set `self.GameDate` (`|MakeArray` (`self.Day`) (`self.Month`) (`self.Year`)))
  (return))

(fn `LoadSavedGameState`
  (returns (IsLoaded :type Boolean))
  (return false))

(fn `NewGameState`
  (`|ExecutionSequence`
    (:`then_0`
      (bind _returnvalue (`DataTableHelper.CreateCountries` "/Game/Data/DataTables/DT_CountriesStats.DT_CountriesStats"))
      (set `self.Countries` _returnvalue))
    (:`then_1`
      (bind _returnvalue_2 (`DataTableHelper.CreateSectors` "/Game/Data/DataTables/DT_AllSectors.DT_AllSectors"))
      (set `self.Sectors` _returnvalue_2))
    (:`then_2`
      (return))))

(fn `Set Time Unit`
  (params (`Game Speed` :type Integer))
  (set `self.TimeUnit` (* (`self.DefaultTimeUnit`) (`|GetArrayItem` (`self.TimeMultipliers`) (- `Game Speed` 1))))
  (return))

(fn `SetCalendar`
  (params (Date :type "Array of Integer (by ref)"))
  (returns (Success :type Boolean))
  (return false))

(fn `SetClock`
  (params (Time :type "Array of Integer (by ref)"))
  (returns (Success :type Boolean))
  (return false))

(fn `SetCountryInfo`
  (params (Country :type "Country Object Reference"))
  (returns (Success :type Boolean))
  (return false))

(fn `StartCalendar`
  (`self.SetActorTickEnabled` true))

(fn `Update Clock`
  (returns (`New Game Time` :type "Array of Integer"))
  (bind (_remainder _returnvalue) (`KismetMathLibrary.FMod` (* (`self.Clockwork`) (`self.SecondsInHour`)) (`self.MinutesInHour`)))
  (bind (_remainder_2 _returnvalue_2) (`KismetMathLibrary.FMod` (`KismetMathLibrary.Conv_IntToDouble` _returnvalue) (`self.SecondsInMinute`)))
  (set `self.Seconds` (`KismetMathLibrary.FFloor` _remainder))
  (set `self.Minutes` (`KismetMathLibrary.FFloor` _remainder_2))
  (set `self.Hours` (`KismetMathLibrary.FFloor` (`KismetMathLibrary.FMod` (`KismetMathLibrary.Conv_IntToDouble` _returnvalue_2) (`self.HoursInDay`))))
  (bind _output_get (set `self.GameTime` (`|MakeArray` (`self.Seconds`) (`self.Minutes`) (`self.Hours`))))
  (return _output_get))

(fn `Update Date`
  (returns (`New Game Date` :type "Array of Integer") (NewMonth :type Boolean))
  (locals (MonthPassed :type Boolean :default false))
  ;[1 1 1] If day passes the max days in month
  (bind _output_get (set `self.Day` (+ (`self.Day`) (`self.DayTick`))))
  (if (> _output_get (`KismetMathLibrary.DaysInMonth` (`self.Year`) (`self.Month`)))
    (set `self.Day` 1) ; Reset day count
    (set `self.Month` (+ (`self.Month`) 1)) ; Inc month
    (set `local.MonthPassed` true))
  ;[1 1 1] If month passes the max months in year
  (if (> (`self.Month`) 12)
    (set `self.Month` 1) ; Inc month
    (set `self.Year` (+ (`self.Year`) 1)))
  (bind _output_get_2 (set `self.GameDate` (`|MakeArray` (`self.Day`) (`self.Month`) (`self.Year`))))
  (return _output_get_2 (`local.MonthPassed`)))

(fn `UserConstructionScript`)