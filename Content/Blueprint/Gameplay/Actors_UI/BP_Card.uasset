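; BP_Card is an actor that shows a card through a WB_Card widget component and lets the player spin it by swiping.
; On BeginPlay it passes CardInfo to the widget and caches the BP_Gameplay_PC controller.
; Touches on the widget open and close a gate on Tick.
; Once a swipe passes the threshold, TouchStart moves far away so rotation continues, applying clamped, inverted horizontal touch deltas as yaw.
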(event `self.ReceiveBeginPlay`
  ;[1 1 1] On Begin Play
  (bind _aswb_card (cast `/Game/Blueprint/UI/Gameplay/Widgets/WB_Card` (`WidgetComponent.GetUserWidgetObject` (`self.Widget`))))
  (set `/Game/Blueprint/UI/Gameplay/Widgets/WB_Card.CardInfo` (`self.CardInfo`) _aswb_card)
  (bind _asbp_gameplay_pc (cast `/Game/Blueprint/Gameplay/BP_Gameplay_PC` (`GameplayStatics.GetPlayerController` 0)))
  (set `self.PlayerControllerRef` _asbp_gameplay_pc))

(event `self.ReceiveTick`
  (params (DeltaSeconds :type "Float (single-precision)"))
  (bind (_locationx _locationy) (`PlayerController.GetInputTouchState` (`self.PlayerControllerRef`) "Touch1"))
  (bind _returnvalue (`KismetMathLibrary.MakeVector2D` _locationx _locationy))
  (bind _returnvalue_x (`KismetMathLibrary.BreakVector2D` (* (- _returnvalue (`self.PriorTouchLoc`)) (`self.SwipeSpeed`))))
  ;[1 1 1] Swipe/Rotating Card
  (`/Engine/EditorBlueprintResources/StandardMacros.Gate` true :!label _label
    (:`Exit`
      (if (>= (`KismetMathLibrary.VSize2D` (- _returnvalue (`self.TouchStart`))) (`self.SwipeThreshold`))
        (set `self.TouchStart` (100000.0 100000.0))
        (`self.K2_AddActorWorldRotation` (`KismetMathLibrary.MakeRotator` 0.0 0.0 (`KismetMathLibrary.FClamp` (* _returnvalue_x -1.0) -10.0 10.0)))
        (set `self.PriorTouchLoc` _returnvalue)))))

(event `self.Widget.OnInputTouchBegin`
  (params (FingerIndex :type "ETouchIndex Enum" :default "Touch1") (TouchedComponent :type "PrimitiveComponent Object Reference"))
  (bind (_locationx _locationy) (`PlayerController.GetInputTouchState` (`self.PlayerControllerRef`) "Touch1"))
  ;[1 1 1] Swipe/Rotating Card
  (`/Engine/EditorBlueprintResources/StandardMacros.IsValid` TouchedComponent
    (:`Is Valid`
      (bind _output_get (set `self.TouchStart` (`KismetMathLibrary.MakeVector2D` _locationx _locationy)))
      (set `self.PriorTouchLoc` _output_get)
      (goto _label :!via `Open`))))

(event `self.Widget.OnInputTouchEnd`
  (params (FingerIndex :type "ETouchIndex Enum" :default "Touch1") (TouchedComponent :type "PrimitiveComponent Object Reference"))
  ;[1 1 1] Swipe/Rotating Card
  (goto _label :!via `Close`))

(fn `UserConstructionScript`)