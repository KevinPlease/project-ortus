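; BP_Country is a map country actor with a mesh, a flag pin and world-space menus for pre-game selection and gameplay.
; Construction applies the mesh, a dynamic M_Country material and the pin offset.
; Pin selection notifies BP_Gameplay_PC according to game phase; pre-game toggles show a details menu and set the IsSelected material parameter.
; When gameplay starts, it destroys the details widget and binds the context menu instead.
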(event `self.ReceiveBeginPlay`
  ;[1 1 1] Event begin play
  (bind _asbp_gameplay_pc (cast `/Game/Blueprint/Gameplay/BP_Gameplay_PC` (`GameplayStatics.GetPlayerController` 0)))
  (set `self.PlayerControllerRef` _asbp_gameplay_pc)
  (`self.Toggle Country Pin` true)
  (`self.Configure Widget` false))

(event `On Country Pin Selected`
  (bind _playercontrollerref (`self.PlayerControllerRef`))
  ;[1 1 1] Country Pin was selected - toggle menus
  (if (`/Game/Blueprint/Gameplay/BP_Gameplay_PC.GameplayStarted` (`self.PlayerControllerRef`))
    (`/Game/Blueprint/Gameplay/BP_Gameplay_PC.Game:On Country Focused` _playercontrollerref self)
    (else
      (`/Game/Blueprint/Gameplay/BP_Gameplay_PC.PreGame:On Country Focused` _playercontrollerref self))))

(event `Game:On Gameplay Started`
  ;[1 1 1] Gameplay has started after picking a country - recreate respective widget
  (set `self.WBContextDetailsMenuRef` null)
  (`ActorComponent.K2_DestroyComponent` (`self.CountryDetailsWidget`))
  (`self.Configure Widget` true))

(event `PreGame:On Country Actor Selected`
  ;[0.5972 0.2831 0.05286] TODO: Country was selected to play with - check if anything needs to be run for this actor specifically
)

(fn `Configure Widget`
  (params (`Has Gameplay Started` :type Boolean))
  (if `Has Gameplay Started`
    (bind _aswb_country_context (cast `/Game/Blueprint/UI/Gameplay/Widgets/Map/WB_CountryContext` (`WidgetComponent.GetUserWidgetObject` (`self.CountryContextWidget`))))
    (bind _output_get (set `self.WBContextMenuRef` _aswb_country_context))
    (set `/Game/Blueprint/UI/Gameplay/Widgets/Map/WB_CountryContext.ParentActor` self _output_get)
    (else
      (bind _aswb_country_context_details (cast `/Game/Blueprint/UI/Gameplay/Widgets/Map/WB_CountryContextDetails` (`WidgetComponent.GetUserWidgetObject` (`self.CountryDetailsWidget`))))
      (bind _output_get_2 (set `self.WBContextDetailsMenuRef` _aswb_country_context_details))
      (set `/Game/Blueprint/UI/Gameplay/Widgets/Map/WB_CountryContextDetails.ParentActor` self _output_get_2))))

(fn `Game:Toggle Country Context Menu`
  (params (IsVisible :type Boolean))
  (if IsVisible
    (`SceneComponent.SetVisibility` (`self.CountryContextWidget`) true false)
    (`/Game/Blueprint/UI/Gameplay/Widgets/Map/WB_CountryContext.Open` (`self.WBContextMenuRef`))
    (else
      (`/Game/Blueprint/UI/Gameplay/Widgets/Map/WB_CountryContext.Close` (`self.WBContextMenuRef`)))))

(fn `PreGame:Toggle Country Details Menu`
  (params (IsVisible :type Boolean))
  (bind _countrydetailswidget (`self.CountryDetailsWidget`))
  (bind _countrydetailswidget_2 (`self.CountryDetailsWidget`))
  ;[1 1 1] PreGame - Country Details
  (`self.PreGame:Toggle Map Selection` IsVisible)
  (if IsVisible
    (`SceneComponent.SetVisibility` _countrydetailswidget_2 true false)
    (`SceneComponent.K2_AddLocalOffset` _countrydetailswidget_2 (0.0 0.0 20.0) false false)
    (`/Game/Blueprint/UI/Gameplay/Widgets/Map/WB_CountryContextDetails.PreGame:On Country Details Selected` (`self.WBContextDetailsMenuRef`) (`self.CountryName`))
    (else
      (`/Game/Blueprint/UI/Gameplay/Widgets/Map/WB_CountryContextDetails.Close` (`self.WBContextDetailsMenuRef`) true)
      (`SceneComponent.SetVisibility` _countrydetailswidget false false)
      (`SceneComponent.K2_AddLocalOffset` _countrydetailswidget (0.0 0.0 -20.0) false false))))

(fn `PreGame:Toggle Map Selection`
  (params (IsSelected :type Boolean))
  (bind _countrystaticmesh (`self.CountryStaticMesh`))
  (if IsSelected
    (`MeshComponent.SetScalarParameterValueOnMaterials` _countrystaticmesh "IsSelected" 0.0) ; Selected
    (else
      (`MeshComponent.SetScalarParameterValueOnMaterials` _countrystaticmesh "IsSelected" 1.0) ; Deselected
    )))

(fn `Toggle Country Pin`
  (params (IsVisible :type Boolean))
  (bind _wbcountrypin (`self.WBCountryPin`))
  (if IsVisible
    (`/Engine/EditorBlueprintResources/StandardMacros.IsValid` (`self.WBCountryPin`)
      (:`Is Valid`
        _)
      (:`Is Not Valid`
        (bind _aswb_country_pin (cast `/Game/Blueprint/UI/Gameplay/Widgets/Map/WB_CountryPin` (`WidgetComponent.GetUserWidgetObject` (`self.CountryPinWidget`))))
        (set `self.WBCountryPin` _aswb_country_pin)
        (set `/Game/Blueprint/UI/Gameplay/Widgets/Map/WB_CountryPin.ParentActor` self _wbcountrypin)
        (set `/Game/Blueprint/UI/Gameplay/Widgets/Map/WB_CountryPin.FlagImage` (`self.CountryFlagIcon`) _wbcountrypin)))
    (`SceneComponent.SetVisibility` (`self.CountryPinWidget`) true false)
    (else
      (`SceneComponent.SetVisibility` (`self.CountryPinWidget`) false false))))

(fn `UserConstructionScript`
  (bind _countrystaticmesh (`self.CountryStaticMesh`))
  (`StaticMeshComponent.SetStaticMesh` _countrystaticmesh (`self.CountryMesh`))
  (bind _returnvalue (`KismetMaterialLibrary.CreateDynamicMaterialInstance` "/Game/Materials/M_Country.M_Country"))
  (`PrimitiveComponent.SetMaterial` _countrystaticmesh 0 _returnvalue)
  (`SceneComponent.K2_AddRelativeLocation` (`self.CountryPinWidget`) (`self.PinLocationOffset`) false false)
  (`PrimitiveComponent.SetCastShadow` (`self.CountryContextWidget`) false)
  (`PrimitiveComponent.SetCastShadow` (`self.CountryDetailsWidget`) false)
  (`PrimitiveComponent.SetCastShadow` (`self.CountryPinWidget`) false))