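; Game mode for a country management game that starts or continues gameplay and links the game state to the player controller.
; A selected country starts the calendar and initializes UI and country actors, while the new-game path is empty.
; It relays date and country selection to the UI, sets game speed, and adds income to country budgets monthly.
; Lookup functions serve sector, service and industry card data, mostly from data tables; calendar, clock and country setters are stubs.
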(event `On Begin Gameplay`
  ;[1 1 1] Gameplay has begun -- either continue or new game
  (`self.Get References`)
  (bind (_country _isselected) (`/Game/Blueprint/Gameplay/BP_Gameplay_GS.GetSelectedCountry` (`self.GameStateRef`)))
  (if _isselected
    (`self.On Continue Game` _country)
    (else
      (`self.On New Game`))))

(event `Update Game Speed`
  (params (`Game Speed` :type Integer))
  ;[1 1 1] Updates the time unit based on game speed selection
  (`/Game/Blueprint/Gameplay/BP_Gameplay_GS.Set Time Unit` (`self.GameStateRef`) `Game Speed`))

(event `Call Player Update DateTime`
  (params (GameDateTime :type "Array of Integer (by ref)"))
  ;[1 1 1] Call player update date - called from game state
  (`/Game/Blueprint/Gameplay/BP_Gameplay_PC.UI Update Date` (`self.PlayerControllerRef`) GameDateTime))

(event `On New Game`
  ;[1 1 1] New Game or Continue with the given country
)

(event `Event Countries Progression - Monthly`
  (bind _countriesstats (`/Game/Blueprint/Gameplay/BP_Gameplay_GS.CountriesStats` (`self.GameStateRef`)))
  ;[0.5972 0.2831 0.05286] TODO: Call Countries progression -- Update UI in the future
  (for (_array_element _array_index) _countriesstats
    (bind _new_country_info (`self.Update Country Budget` _array_element)
      (:`End`
        (`KismetArrayLibrary.Array_Set` _countriesstats _array_index _new_country_info)))))

(event `On Continue Game`
  (params (SelectedCountry :type "CountryStruct Structure"))
  ;[1 1 1] New Game or Continue with the given country
  (`/Game/Blueprint/Gameplay/BP_Gameplay_GS.StartCalendar` (`self.GameStateRef`))
  (`/Game/Blueprint/Gameplay/BP_Gameplay_PC.On Begin Gameplay` (`self.PlayerControllerRef`) SelectedCountry)
  (`self.Game:UpdateCountryActors`))

(event `On Country Selected`
  (params (`Country Name` :type String))
  ;[1 1 1] Country was selected in the map - Get info - Update UI
  (`/Game/Blueprint/Gameplay/BP_Gameplay_PC.UI Update Status Bar` (`self.PlayerControllerRef`) (`self.GetCountryInfoByName` `Country Name`)))

(fn `Game:UpdateCountryActors`
  (for _array_element (`self.AllCountryActors`)
    (`/Game/Blueprint/Gameplay/Actors_UI/BP_Country.Game:On Gameplay Started` _array_element)))

(fn `Get Cards For SubService`
  (params (Industry :type "/Game/Data/Enums/Enum_Industries Enum" :default "NewEnumerator0"))
  (returns (CardsList :type "Array of CardInfo Structure"))
  (locals (CardsInfo :type "Array of CardInfo Structure"))
  (switch `/Game/Data/Enums/Enum_Industries` Industry
    (:`NewEnumerator0`
      (bind _returnvalue (`DataTableHelper.GetCardsInfoFromDataTable` "/Game/Data/DataTables/BasicServices/DT_CardsInfo_Power.DT_CardsInfo_Power"))
      (set `local.CardsInfo` _returnvalue))
    (:`NewEnumerator1`
      (bind _returnvalue_2 (`DataTableHelper.GetCardsInfoFromDataTable` "/Game/Data/DataTables/BasicServices/DT_CardsInfo_Water.DT_CardsInfo_Water"))
      (set `local.CardsInfo` _returnvalue_2))
    (:`NewEnumerator2`
      (bind _returnvalue_3 (`DataTableHelper.GetCardsInfoFromDataTable` "/Game/Data/DataTables/BasicServices/DT_CardsInfo_Waste.DT_CardsInfo_Waste"))
      (set `local.CardsInfo` _returnvalue_3))
    (:`NewEnumerator3`
      (bind _returnvalue_4 (`DataTableHelper.GetCardsInfoFromDataTable` "/Game/Data/DataTables/BasicServices/DT_CardsInfo_Transport.DT_CardsInfo_Transport"))
      (set `local.CardsInfo` _returnvalue_4))
    (:`NewEnumerator4`
      (bind _returnvalue_5 (`DataTableHelper.GetCardsInfoFromDataTable` "/Game/Data/DataTables/BasicServices/DT_CardsInfo_Landscape.DT_CardsInfo_Landscape"))
      (set `local.CardsInfo` _returnvalue_5))
    (:`NewEnumerator5`
      (bind _returnvalue_6 (`DataTableHelper.GetCardsInfoFromDataTable` "/Game/Data/DataTables/BasicServices/DT_CardsInfo_Information.DT_CardsInfo_Information"))
      (set `local.CardsInfo` _returnvalue_6)))
  (return (`local.CardsInfo`)))

(fn `Get References`
  (bind _asbp_gameplay_pc (cast `/Game/Blueprint/Gameplay/BP_Gameplay_PC` (`GameplayStatics.GetPlayerController` 0)))
  (set `self.PlayerControllerRef` _asbp_gameplay_pc)
  (bind _asbp_gameplay_gs (cast `/Game/Blueprint/Gameplay/BP_Gameplay_GS` (`GameplayStatics.GetGameState`)))
  (set `self.GameStateRef` _asbp_gameplay_gs)
  (return))

(fn `Get Services For Sector`
  (params (SelectionSector :type "/Game/Data/Enums/Enum_Sectors Enum" :default "NewEnumerator0"))
  (returns (Services :type "Array of ServiceStruct Structure"))
  (locals (ServicesInfo :type "Array of ServiceStruct Structure"))
  (switch `/Game/Data/Enums/Enum_Sectors` SelectionSector
    (:`NewEnumerator0`
      (bind _returnvalue (`DataTableHelper.GetServicesInfoFromDataTable` "/Game/Data/DataTables/DT_PublicSector_Services.DT_PublicSector_Services"))
      (set `local.ServicesInfo` _returnvalue)
      (return (`local.ServicesInfo`)))))

(fn `Get SubServices For Service`
  (params (ServiceTitle :type String))
  (returns (Services :type "Array of ServiceStruct Structure"))
  (locals (ServicesInfo :type "Array of ServiceStruct Structure"))
  (bind _returnvalue (`DataTableHelper.GetSubServicesInfoForService` ServiceTitle))
  (return _returnvalue))

(fn `GetCountryInfoByName`
  (params (Name :type String))
  (returns (Country :type "CountryStruct Structure"))
  (bind _country (`/Game/Blueprint/Gameplay/BP_Gameplay_GS.Get Info For Country` (`self.GameStateRef`) Name))
  (return _country))

(fn `SetCalendar`
  (params (Date :type "Array of Integer (by ref)"))
  (returns (Success :type Boolean))
  (return false))

(fn `SetClock`
  (params (Time :type "Array of Integer (by ref)"))
  (returns (Success :type Boolean))
  (return false))

(fn `SetCountryInfo`
  (params (`Country Struct` :type "CountryStruct Structure"))
  (returns (Success :type Boolean))
  (return false))

(fn `UserConstructionScript`)