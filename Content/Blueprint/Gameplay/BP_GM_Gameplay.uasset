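; Gameplay game mode for a country-management game with sectors, industries and cards, linking the game state to the main HUD.
; On begin play it caches the controller and game state and creates the HUD, then relays date and game-speed changes.
; Country progression adds income to each country's budget and refreshes the HUD list.
; Getters read data tables; only Public Sector has industries, and calendar, clock and country-info setters are stubs.
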(event `Event Countries Progression`
  (bind _countriesstats (`/Game/Blueprint/Gameplay/BP_GS_Gameplay.CountriesStats` (`self.GameStateRef`)))
  ;[1 1 1] Call Countries progression
  (for (_array_element _array_index) _countriesstats
    (bind _new_country_info (`self.Update Country Struct` _array_element)
      (:`End`
        (`KismetArrayLibrary.Array_Set` _countriesstats _array_index _new_country_info))))
  (`self.UI Update Countries List` _countriesstats))

(event `self.ReceiveBeginPlay`
  ;[1 1 1] Begin game - Get References
  (`self.Get References`)
  (`self.Init HUD`))

(event `Update Game Speed`
  (params (`Game Speed` :type Integer))
  ;[1 1 1] Updates the time unit based on game speed selection
  (`/Game/Blueprint/Gameplay/BP_GS_Gameplay.Set Time Unit` (`self.GameStateRef`) `Game Speed`))

(event `Init HUD`
  ;[1 1 1] Init/Setup main HUD
  (bind _returnvalue (`|CreateWidget` "/Game/Blueprint/UI/Gameplay/HUD/WB_HUDMain.WB_HUDMain_C" (`self.PlayerControllerRef`)))
  (bind _output_get (set `self.HUDMainRef` _returnvalue))
  (`UserWidget.AddToViewport` _output_get 0))

(event `UI Update Date`
  (params (GameDate :type "Array of Integer"))
  ;[1 1 1] Update Date UI
  (message `/Game/Blueprint/UI/I_HUDMain.SetCalendar` (`self.HUDMainRef`) GameDate))

(event `UI Update Countries List`
  (params (`List of country stats` :type "Array of CountryStruct Structure"))
  ;[1 1 1] Update the list of countries UI
  (`/Game/Blueprint/UI/Gameplay/HUD/WB_HUDMain.Init Countries List` (`self.HUDMainRef`) `List of country stats`))

(fn `Get All Sectors`
  (returns (Sectors :type "Array of SectorStruct Structure"))
  (locals (IndustriesInfo :type "Array of IndustryStruct Structure"))
  (bind _returnvalue (`DataTableHelper.GetSectorsInfoFromDataTable` "/Game/Data/DataTables/DT_AllSectors.DT_AllSectors"))
  (return _returnvalue))

(fn `Get Cards For Industry`
  (params (Industry :type "/Game/Data/Enums/Enum_Industries Enum" :default "NewEnumerator0"))
  (returns (CardsList :type "Array of CardInfo Structure"))
  (locals (CardsInfo :type "Array of CardInfo Structure"))
  (switch `/Game/Data/Enums/Enum_Industries` Industry
    (:`NewEnumerator0`
      (bind _returnvalue (`DataTableHelper.GetCardsInfoFromDataTable` "/Game/Data/DataTables/PublicSector/DT_CardsInfo_Power.DT_CardsInfo_Power"))
      (set `local.CardsInfo` _returnvalue))
    (:`NewEnumerator1`
      (bind _returnvalue_2 (`DataTableHelper.GetCardsInfoFromDataTable` "/Game/Data/DataTables/PublicSector/DT_CardsInfo_Water.DT_CardsInfo_Water"))
      (set `local.CardsInfo` _returnvalue_2))
    (:`NewEnumerator2`
      (bind _returnvalue_3 (`DataTableHelper.GetCardsInfoFromDataTable` "/Game/Data/DataTables/PublicSector/DT_CardsInfo_Waste.DT_CardsInfo_Waste"))
      (set `local.CardsInfo` _returnvalue_3))
    (:`NewEnumerator3`
      (bind _returnvalue_4 (`DataTableHelper.GetCardsInfoFromDataTable` "/Game/Data/DataTables/PublicSector/DT_CardsInfo_Transport.DT_CardsInfo_Transport"))
      (set `local.CardsInfo` _returnvalue_4))
    (:`NewEnumerator4`
      (bind _returnvalue_5 (`DataTableHelper.GetCardsInfoFromDataTable` "/Game/Data/DataTables/PublicSector/DT_CardsInfo_Landscape.DT_CardsInfo_Landscape"))
      (set `local.CardsInfo` _returnvalue_5))
    (:`NewEnumerator5`
      (bind _returnvalue_6 (`DataTableHelper.GetCardsInfoFromDataTable` "/Game/Data/DataTables/PublicSector/DT_CardsInfo_Information.DT_CardsInfo_Information"))
      (set `local.CardsInfo` _returnvalue_6)))
  (return (`local.CardsInfo`)))

(fn `Get Industries For Sector`
  (params (Sector :type String))
  (returns (ReturnValue :type "Array of IndustryStruct Structure"))
  (locals (IndustriesInfo :type "Array of IndustryStruct Structure"))
  (switch `string` Sector
    (:`Public Sector`
      (bind _returnvalue (`DataTableHelper.GetIndustriesInfoFromDataTable` "/Game/Data/DataTables/PublicSector/DT_SectorInfo_Public.DT_SectorInfo_Public"))
      (set `local.IndustriesInfo` _returnvalue)
      (return (`local.IndustriesInfo`)))))

(fn `Get References`
  (bind _asbp_pc_gameplay (cast `/Game/Blueprint/Gameplay/BP_PC_Gameplay` (`GameplayStatics.GetPlayerController` 0)))
  (set `self.PlayerControllerRef` _asbp_pc_gameplay)
  (bind _asbp_gs_gameplay (cast `/Game/Blueprint/Gameplay/BP_GS_Gameplay` (`GameplayStatics.GetGameState`)))
  (set `self.GameStateRef` _asbp_gs_gameplay)
  (return))

(fn `SetCalendar`
  (params (Date :type "Array of Integer (by ref)"))
  (returns (Success :type Boolean))
  (return false))

(fn `SetClock`
  (params (Time :type "Array of Integer (by ref)"))
  (returns (Success :type Boolean))
  (return false))

(fn `SetCountryInfo`
  (params (`Country Struct` :type "CountryStruct Structure"))
  (returns (Success :type Boolean))
  (return false))

(fn `UserConstructionScript`)