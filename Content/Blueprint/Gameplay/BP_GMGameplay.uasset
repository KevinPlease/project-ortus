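; Gameplay game mode that sets up the main HUD and relays between UI, game state and card data.
; On BeginPlay it caches the gameplay player controller and game state, then creates the HUD widget.
; Events push the date to the HUD calendar and pass game speed to the game state as its time unit.
; Card lookup selects a data table per industry; the industries-per-sector lookup is an unfinished stub.
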(event Custom|Init%20HUD
  ;[1 1 1] Init/Setup main HUD
  (bind _returnvalue (UserInterface|CreateWidget "/Game/Blueprint/UI/Gameplay/WB_HUDMain.WB_HUDMain_C" (Variables|References|GetPlayerControllerRef)))
  (bind _output_get (Variables|UIReferences|SetHUDMainRef _returnvalue))
  (UserInterface|Viewport|AddtoViewport _output_get 0))

(event Custom|UI%20Update%20Date
  (params (GameDate :type Array%20of%20Integers))
  ;[1 1 1] Update Date UI
  (Class|IHUDMain|SetCalendar(Message) (Variables|UIReferences|GetHUDMainRef) GameDate))

(event Custom|Update%20Game%20Speed
  (params (Game%20Speed :type Integer))
  ;[1 1 1] Updates the time unit based on game speed selection
  (Default|SetTimeUnit (Variables|References|GetGameStateRef) Game%20Speed))

(event EventBeginPlay
  ;[1 1 1] Begin game - Get References
  (CallFunction|GetReferences)
  (CallFunction|InitHUD))

(fn ConstructionScript)

(fn GetReferences
  (bind _asbp_pcgameplay (Utilities|Casting|CastToBP_PCGameplay (Game|GetPlayerController 0)))
  (Variables|References|SetPlayerControllerRef _asbp_pcgameplay)
  (bind _asbp_gsgameplay (Utilities|Casting|CastToBP_GSGameplay (Game|GetGameState)))
  (Variables|References|SetGameStateRef _asbp_gsgameplay)
  (return))

(fn GetCardsInfoforIndustry
  (params (Industry :type Enum_Industries%20Enum :default "NewEnumerator0"))
  (switch Utilities|FlowControl|Switch|SwitchonEnum_Industries Industry
    (:NewEnumerator0
      (bind _returnvalue (Class|DataTableHelper|GetCardsInfofromDataTable "/Game/Data/DataTables/DT_CardsInfo_Power.DT_CardsInfo_Power"))
      (LocalVariables|SetCardsInfo _returnvalue))
    (:NewEnumerator1
      (bind _returnvalue_2 (Class|DataTableHelper|GetCardsInfofromDataTable "/Game/Data/DataTables/DT_CardsInfo_Water.DT_CardsInfo_Water"))
      (LocalVariables|SetCardsInfo _returnvalue_2))
    (:NewEnumerator2
      (bind _returnvalue_3 (Class|DataTableHelper|GetCardsInfofromDataTable "/Game/Data/DataTables/DT_CardsInfo_Waste.DT_CardsInfo_Waste"))
      (LocalVariables|SetCardsInfo _returnvalue_3))
    (:NewEnumerator3
      (bind _returnvalue_4 (Class|DataTableHelper|GetCardsInfofromDataTable "/Game/Data/DataTables/DT_CardsInfo_Transport.DT_CardsInfo_Transport"))
      (LocalVariables|SetCardsInfo _returnvalue_4))
    (:NewEnumerator4
      (bind _returnvalue_5 (Class|DataTableHelper|GetCardsInfofromDataTable "/Game/Data/DataTables/DT_CardsInfo_Landscape.DT_CardsInfo_Landscape"))
      (LocalVariables|SetCardsInfo _returnvalue_5))
    (:NewEnumerator5
      (bind _returnvalue_6 (Class|DataTableHelper|GetCardsInfofromDataTable "/Game/Data/DataTables/DT_CardsInfo_Information.DT_CardsInfo_Information"))
      (LocalVariables|SetCardsInfo _returnvalue_6)))
  (return (LocalVariables|GetCardsInfo)))

(fn GetIndustriesInfoforSector
  (params (Sector :type Enum_Sectors%20Enum :default "NewEnumerator0"))
  (switch Utilities|FlowControl|Switch|SwitchonEnum_Sectors Sector))