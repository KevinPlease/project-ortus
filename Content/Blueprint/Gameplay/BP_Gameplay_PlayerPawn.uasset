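; Player pawn that pans by one-finger touch swipe, moving along world Y and Z with horizontal input inverted.
; A Finger1 press records the touch start if movement is enabled and opens a Tick gate, which release closes.
; Once the swipe passes a threshold, the start point jumps far away to keep the check true, and per-frame touch deltas scaled by swipe speed feed movement input.
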(event `self.ReceiveBeginPlay`
  ;[1 1 1] Being play - Get Refernces
  (bind _asbp_gameplay_pc (cast `/Game/Blueprint/Gameplay/BP_Gameplay_PC` (`GameplayStatics.GetPlayerController` 0)))
  (set `self.PlayerControllerRef` _asbp_gameplay_pc))

(event `self.ReceiveTick`
  (params (DeltaSeconds :type "Float (single-precision)"))
  (bind (_locationx _locationy) (`PlayerController.GetInputTouchState` (`self.PlayerControllerRef`) "Touch1"))
  (bind _returnvalue (`KismetMathLibrary.MakeVector2D` _locationx _locationy))
  (bind (_returnvalue_x _returnvalue_y) (`KismetMathLibrary.BreakVector2D` (* (- _returnvalue (`self.PriorTouchLoc`)) (`self.SwipeSpeed`))))
  ;[1 1 1] Swipe to pan input
  (`/Engine/EditorBlueprintResources/StandardMacros.Gate` true :!label _label
    (:`Exit`
      (if (>= (`KismetMathLibrary.VSize2D` (- _returnvalue (`self.TouchStart`))) (`self.SwipeThreshold`))
        (set `self.TouchStart` (100000.0 100000.0))
        (`self.AddMovementInput` (`KismetMathLibrary.MakeVector` 0.0 (* _returnvalue_x -1.0) _returnvalue_y))
        (set `self.PriorTouchLoc` _returnvalue)))))

(event `InputAction|Finger1`
  (params (Key :type "Key Structure"))
  (bind (_locationx _locationy) (`PlayerController.GetInputTouchState` (`self.PlayerControllerRef`) "Touch1"))
  ;[1 1 1] Swipe to pan input
  (:`Pressed`
    (if (`self.IsMovementEnabled`)
      (bind _output_get (set `self.TouchStart` (`KismetMathLibrary.MakeVector2D` _locationx _locationy)))
      (set `self.PriorTouchLoc` _output_get)
      (goto _label :!via `Open`)))
  (:`Released`
    (goto _label :!via `Close`)))

(fn `UserConstructionScript`)