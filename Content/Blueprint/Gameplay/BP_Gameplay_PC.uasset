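; Player controller for the gameplay map that handles country selection.
; On BeginPlay it caches the gameplay game mode and sets input to Game and UI.
; OnCountrySelected deselects the previously selected country actor, highlights the new one, then forwards its country name to the game mode.
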(event `self.ReceiveBeginPlay`
  ;[1 1 1] Begin Play
  (bind _asbp_gameplay_gm (cast `/Game/Blueprint/Gameplay/BP_Gameplay_GM` (`GameplayStatics.GetGameMode`)))
  (set `self.GameModeRef` _asbp_gameplay_gm)
  (`WidgetBlueprintLibrary.SetInputMode_GameAndUIEx` self null))

(event `On Country Selected`
  (params (CountryActor :type "/Game/Blueprint/Gameplay/Actors_UI/BP_Country Object Reference"))
  (bind _previousselectedactor (`self.PreviousSelectedActor`))
  (bind _currentlyselectedactor (`self.CurrentlySelectedActor`))
  ;[1 1 1] Country Selection on the Map -- Update Visuals
  (set `self.CurrentlySelectedActor` CountryActor)
  (`/Engine/EditorBlueprintResources/StandardMacros.IsValid` _previousselectedactor
    (:`Is Valid`
      (`/Game/Blueprint/Gameplay/Actors_UI/BP_Country.ToggleSelection` _previousselectedactor false) ; Deselect previous country
    )
    (:`Is Not Valid`
      _))
  (`/Game/Blueprint/Gameplay/Actors_UI/BP_Country.ToggleSelection` _currentlyselectedactor true) ; Select country
  (bind _output_get (set `self.PreviousSelectedActor` _currentlyselectedactor))
  ;[1 1 1] Call GM with the country selected
  (`/Game/Blueprint/Gameplay/BP_Gameplay_GM.On Country Selected` (`self.GameModeRef`) (`/Game/Blueprint/Gameplay/Actors_UI/BP_Country.CountryName` _output_get)))

(fn `UserConstructionScript`)